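; Blueprint library for the achievement system, covering setup from DT_Achievements, progress and unlocking, list display and menu toggling.
; UnlockAchievement adds progress to a named, unachieved entry, timestamps and saves it, showing a notification and playing a sound on completion.
; GenerateAchievementsList rebuilds entry widgets, collapsing locked secret achievements into one remaining-count widget.
; Live menu and notification widgets are found by class, so callers need no references to them.
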(fn InitiateAchievements
  (bind _outrownames (DataTable|GetDataTableRowNames "/Game/AchievementSystem/DataTables/DT_Achievements.DT_Achievements"))
  (for _array_element _outrownames
    (bind _returnvalue (Utilities|GetDataTableRow "/Game/AchievementSystem/DataTables/DT_Achievements.DT_Achievements" _array_element)
      (:then
        (Utilities|Array|Add (LocalVariables|GetAchievementsList) _returnvalue))))
  (return (LocalVariables|GetAchievementsList)))

(fn GenerateAchievementsList
  (params (Achievements :type Array%20of%20S%20Achievement%20Information%20Structures) (Achievements%20Container :type Panel%20Widget%20Object%20Reference))
  (bind _number_of_achievements_left (LocalVariables|GetNumber%20Of%20Achievements%20Left))
  (Widget|Panel|ClearChildren Achievements%20Container)
  (for _array_element Achievements
    (if (.IsSecret? (Utilities|Struct|BreakS_AchievementInformation _array_element))
      (Math|Integer|IncrementInt (LocalVariables|GetNumber%20Of%20Achievements%20Left)
        (:%20%20
          (if (.IsAchieved? (Utilities|Struct|BreakS_AchievementInformation _array_element))
            (Math|Integer|DecrementInt (LocalVariables|GetNumber%20Of%20Achievements%20Left)
              (:%20%20
                (bind _returnvalue (UserInterface|CreateWidget "/Game/AchievementSystem/Blueprints/UI/AchievementListing/Components/WB_AchievementListed.WB_AchievementListed_C" 0 _array_element))
                (Widget|Panel|AddChild Achievements%20Container _returnvalue))))))
      (else
        (bind _returnvalue_2 (UserInterface|CreateWidget "/Game/AchievementSystem/Blueprints/UI/AchievementListing/Components/WB_AchievementListed.WB_AchievementListed_C" 0 _array_element))
        (Widget|Panel|AddChild Achievements%20Container _returnvalue_2))))
  (if (> _number_of_achievements_left 0)
    (bind _returnvalue_3 (UserInterface|CreateWidget "/Game/AchievementSystem/Blueprints/UI/AchievementListing/Components/WB_SecretAchievementsListed.WB_SecretAchievementsListed_C" 0 _number_of_achievements_left))
    (Widget|Panel|AddChild Achievements%20Container _returnvalue_3)
    (return)))

(fn UnlockAchievement
  (params (Achievement :type Text) (Progression%20to%20Add :type Integer))
  (bind (_date _time) (CallFunction|GetDateandTime))
  (bind (_date_2 _time_2) (CallFunction|GetDateandTime))
  (bind _achievements (CallFunction|LoadAchievements))
  (for (_array_element _array_index) _achievements
    (if (Utilities|Enum|Equal(Enum) Achievement (.Name (Utilities|Struct|BreakS_AchievementInformation _array_element)))
      (if (not (.IsAchieved? (Utilities|Struct|BreakS_AchievementInformation _array_element)))
        (if (>= (+ (.CurrentProgression (Utilities|Struct|BreakS_AchievementInformation _array_element)) Progression%20to%20Add) (.MaximumProgression (Utilities|Struct|BreakS_AchievementInformation _array_element)))
          (bind _returnvalue (UserInterface|CreateWidget "/Game/AchievementSystem/Blueprints/UI/AchievementNotifications/WB_AchievementNotification.WB_AchievementNotification_C" 0 _array_element))
          (bind _foundwidgets (Widget|GetAllWidgetsOfClass 0 "/Game/AchievementSystem/Blueprints/UI/AchievementNotifications/WB_AchievementNotificationListing.WB_AchievementNotificationListing_C" false))
          (for _array_element_2 _foundwidgets
            (Widget|Panel|AddChild (Variables|/Game/AchievementSystem/Blueprints/UI/AchievementNotifications/WB_AchievementNotificationListing.WB_AchievementNotificationListing_C|GetAchievementNotificationContainer _array_element_2) _returnvalue))
          (bind _returnvalue_2 (Utilities|GetDataTableRow "/Game/AchievementSystem/DataTables/DT_AcievementSystemCustomization.DT_AcievementSystemCustomization" "Information")
            (:then
              (if (.IsSecret? (Utilities|Struct|BreakS_AchievementInformation _array_element))
                (Audio|PlaySound2D 0 (.secretachievementachievedsound _returnvalue_2) 1.0 1.0 0.0 0 0)
                (else
                  (Audio|PlaySound2D 0 (.achievementachievedsound _returnvalue_2) 1.0 1.0 0.0 0 0)))
              (bind _structout (Utilities|Struct|SetmembersinS_AchievementInformation _array_element (.IsSecret? (Utilities|Struct|BreakS_AchievementInformation _array_element)) (.UnachievedColor (Utilities|Struct|BreakS_AchievementInformation _array_element)) (.AchievedColor (Utilities|Struct|BreakS_AchievementInformation _array_element)) (+ (.CurrentProgression (Utilities|Struct|BreakS_AchievementInformation _array_element)) Progression%20to%20Add) true _date_2 _time_2))
              (Utilities|Array|SetArrayElem _achievements _array_index _structout)))
          (else
            (bind _structout_2 (Utilities|Struct|SetmembersinS_AchievementInformation _array_element (.IsSecret? (Utilities|Struct|BreakS_AchievementInformation _array_element)) (.UnachievedColor (Utilities|Struct|BreakS_AchievementInformation _array_element)) (.AchievedColor (Utilities|Struct|BreakS_AchievementInformation _array_element)) (+ (.CurrentProgression (Utilities|Struct|BreakS_AchievementInformation _array_element)) Progression%20to%20Add) (>= (+ (.CurrentProgression (Utilities|Struct|BreakS_AchievementInformation _array_element)) Progression%20to%20Add) (.MaximumProgression (Utilities|Struct|BreakS_AchievementInformation _array_element))) _date _time))
            (Utilities|Array|SetArrayElem _achievements _array_index _structout_2)))
        (CallFunction|SaveAchievements _achievements)
        (bind _foundwidgets_2 (Widget|GetAllWidgetsOfClass 0 "/Game/AchievementSystem/Blueprints/UI/AchievementListing/WB_AchievementsListMenu.WB_AchievementsListMenu_C" false))
        (for _array_element_3 _foundwidgets_2
          (CallFunction|GenerateAchievementsList _achievements (Variables|/Game/AchievementSystem/Blueprints/UI/AchievementListing/WB_AchievementsListMenu.WB_AchievementsListMenu_C|GetAchievementsContainer _array_element_3)))))))

(fn Show/HideAchievementsListMenu
  (bind _returnvalue (Game|GetPlayerController 0))
  (bind _foundwidgets (Widget|GetAllWidgetsOfClass 0 "/Game/AchievementSystem/Blueprints/UI/AchievementListing/WB_AchievementsListMenu.WB_AchievementsListMenu_C" false))
  (for _array_element _foundwidgets
    (if (Variables|/Game/AchievementSystem/Blueprints/UI/AchievementListing/WB_AchievementsListMenu.WB_AchievementsListMenu_C|GetCanPressAgain _array_element)
      (Variables|/Game/AchievementSystem/Blueprints/UI/AchievementListing/WB_AchievementsListMenu.WB_AchievementsListMenu_C|SetCanPressAgain _array_element false)
      (if (Widget|IsVisible _array_element)
        (Default|PlayAnimation _array_element false)
        (Variables|/Script/Engine.PlayerController|SetbShowMouseCursor _returnvalue true)
        (Input|SetInputModeGameOnly _returnvalue false)
        (else
          (Widget|SetVisibility _array_element "SelfHitTestInvisible")
          (Variables|/Script/Engine.PlayerController|SetbShowMouseCursor _returnvalue true)
          (Input|SetInputModeGameandUI _returnvalue _array_element "DoNotLock" false false)
          (Default|PlayAnimation _array_element true))))))

(fn GetDateandTime
  (bind _returnvalue (Math|DateTime|Now))
  (bind _returnvalue_2 (Class|KismetTextLibrary|AsTimeDateTime _returnvalue))
  (bind _returnvalue_3 (Utilities|String|ToString(Text) _returnvalue_2))
  (bind _output_get (LocalVariables|SetLastIndexes (Utilities|String|GetSubstring _returnvalue_3 (- (Utilities|String|Len _returnvalue_3) 2) 2)))
  (return (Utilities|String|ToString(Text) (Class|KismetTextLibrary|AsDateDateTime _returnvalue)) (Utilities|String|Append (Utilities|String|LeftChop _returnvalue_3 6) " " _output_get)))