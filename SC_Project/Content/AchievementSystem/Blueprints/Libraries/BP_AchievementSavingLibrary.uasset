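; Blueprint function library that saves and loads the achievement system's progress through a BP_AchievementsSave save game.
; The slot name comes from the DT_AcievementSystemCustomization data table.
; When no save exists, it creates and saves one seeded from InitiateAchievements with zero progress.
; Loading also appends achievements missing from an existing save by name, then rebuilds any WB_AchievementsListMenu lists and returns the array.
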(fn SaveAchievements
  (params (Achievements :type Array%20of%20S%20Achievement%20Information%20Structures))
  (bind _returnvalue (Utilities|GetDataTableRow "/Game/AchievementSystem/DataTables/DT_AcievementSystemCustomization.DT_AcievementSystemCustomization" "Information")
    (:then
      (bind _achievements_save_object (CallFunction|GetAchievementSaveObject))
      (Variables|/Game/AchievementSystem/Blueprints/SaveGame/BP_AchievementsSave.BP_AchievementsSave_C|SetAchievements _achievements_save_object Achievements)
      (SaveGame|SaveGametoSlot _achievements_save_object (.achievementssavefilename _returnvalue))
      (return))))

(fn LoadAchievements
  (bind _returnvalue (Utilities|GetDataTableRow "/Game/AchievementSystem/DataTables/DT_AcievementSystemCustomization.DT_AcievementSystemCustomization" "Information")
    (:then
      (bind _returnvalue_2 (SaveGame|DoesSaveGameExist (.achievementssavefilename _returnvalue)))
      (if _returnvalue_2
        (bind _returnvalue_3 (SaveGame|LoadGamefromSlot (.achievementssavefilename _returnvalue)))
        (bind _achievement_list (CallFunction|InitiateAchievements))
        (for _array_element _achievement_list
          (bind _asbp_achievements_save (Utilities|Casting|CastToBP_AchievementsSave _returnvalue_3))
          (LocalVariables|SetFound false)
          (for _array_element_2 (Variables|/Game/AchievementSystem/Blueprints/SaveGame/BP_AchievementsSave.BP_AchievementsSave_C|GetAchievements _asbp_achievements_save)
            (if (Utilities|Enum|Equal(Enum) (.Name (Utilities|Struct|BreakS_AchievementInformation _array_element_2)) (stale _achievement_name))
              (LocalVariables|SetFound true)))
          (if (not (LocalVariables|GetFound))
            (bind _achievement_name (|GetInformation _array_element (Variables|/Game/AchievementSystem/Blueprints/SaveGame/BP_AchievementsSave.BP_AchievementsSave_C|GetAchievements _asbp_achievements_save)))))
        (bind _foundwidgets (Widget|GetAllWidgetsOfClass 0 "/Game/AchievementSystem/Blueprints/UI/AchievementListing/WB_AchievementsListMenu.WB_AchievementsListMenu_C" false))
        (for _array_element_3 _foundwidgets
          (CallFunction|GenerateAchievementsList (Variables|/Game/AchievementSystem/Blueprints/SaveGame/BP_AchievementsSave.BP_AchievementsSave_C|GetAchievements _asbp_achievements_save) (Variables|/Game/AchievementSystem/Blueprints/UI/AchievementListing/WB_AchievementsListMenu.WB_AchievementsListMenu_C|GetAchievementsContainer _array_element_3))
          (return (Variables|/Game/AchievementSystem/Blueprints/SaveGame/BP_AchievementsSave.BP_AchievementsSave_C|GetAchievements _asbp_achievements_save)))
        (else
          (bind _returnvalue_4 (SaveGame|CreateSaveGameObject "/Game/AchievementSystem/Blueprints/SaveGame/BP_AchievementsSave.BP_AchievementsSave_C"))
          (bind _achievement_list_2 (CallFunction|InitiateAchievements))
          (for _array_element_4 _achievement_list_2
            (Utilities|Array|Add (Variables|/Game/AchievementSystem/Blueprints/SaveGame/BP_AchievementsSave.BP_AchievementsSave_C|GetAchievements _returnvalue_4) (Utilities|Struct|MakeS_AchievementInformation (.name _array_element_4) (.message _array_element_4) (.issecret? _array_element_4) (.unachievedcolor _array_element_4) (.achievedcolor _array_element_4) (.unachievedicon _array_element_4) (.achievedicon _array_element_4) 0 (.maximumprogression _array_element_4) false "" "")))
          (SaveGame|SaveGametoSlot _returnvalue_4 (.achievementssavefilename _returnvalue))
          (return (Variables|/Game/AchievementSystem/Blueprints/SaveGame/BP_AchievementsSave.BP_AchievementsSave_C|GetAchievements _returnvalue_4)))))))

(fn GetAchievementSaveObject
  (bind _returnvalue (Utilities|GetDataTableRow "/Game/AchievementSystem/DataTables/DT_AcievementSystemCustomization.DT_AcievementSystemCustomization" "Information")
    (:then
      (bind _returnvalue_2 (SaveGame|DoesSaveGameExist (.achievementssavefilename _returnvalue)))
      (if _returnvalue_2
        (bind _returnvalue_3 (SaveGame|LoadGamefromSlot (.achievementssavefilename _returnvalue)))
        (bind _asbp_achievements_save (Utilities|Casting|CastToBP_AchievementsSave _returnvalue_3))
        (return _asbp_achievements_save)
        (else
          (bind _returnvalue_4 (SaveGame|CreateSaveGameObject "/Game/AchievementSystem/Blueprints/SaveGame/BP_AchievementsSave.BP_AchievementsSave_C"))
          (bind _achievement_list (CallFunction|InitiateAchievements _returnvalue_4))
          (for _array_element _achievement_list
            (Utilities|Array|Add (Variables|/Game/AchievementSystem/Blueprints/SaveGame/BP_AchievementsSave.BP_AchievementsSave_C|GetAchievements _returnvalue_4) (Utilities|Struct|MakeS_AchievementInformation (.name _array_element) (.message _array_element) (.issecret? _array_element) (.unachievedcolor _array_element) (.achievedcolor _array_element) (.unachievedicon _array_element) (.achievedicon _array_element) 0 (.maximumprogression _array_element) false "" "")))
          (SaveGame|SaveGametoSlot _returnvalue_4 (.achievementssavefilename _returnvalue))
          (return _returnvalue_4))))))