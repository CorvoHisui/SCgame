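; Farm tile actor that the player interacts with to plant the seed in the selected action-bar slot, or to harvest a full-grown crop.
; GrowPlant advances the stage using Paper2D sprites for wheat or eggplant, and BeginPlay binds to the GameInstance's day-ended event.
; Harvest spawns crop and chance-based seed pickups, then resets the tile.
; Planting, growth and harvest append tile state to the GameInstance save array; SpawnFromSave restores it.
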(event Custom|EventPlantSeed
  (if (not (Variables|Default|GetIsPlanted))
    (bind _asbp_sccharacter (Utilities|Casting|CastToBP_SCCharacter (Game|GetPlayerCharacter 0)))
    (bind _asbp_seed_base (Utilities|Casting|CastToBP_SeedBaseClass (.Item (Default|GetItemInfoatIndex (Variables|/Game/Blueprints/Player/BP_SCCharacter.BP_SCCharacter_C|GetActionBar1 _asbp_sccharacter) (Variables|/Game/Blueprints/Player/BP_SCCharacter.BP_SCCharacter_C|GetSelectedSlot _asbp_sccharacter)))))
    (bind _output_get (Variables|Default|SetSeed _asbp_seed_base))
    (Variables|GrowthVariables|SetTotalTimeToGrow (.TotalTimeToGrow (Utilities|GetClassDefaults _output_get)))
    (Variables|GrowthVariables|SetTotalPlantStages (.PlantStages (Utilities|GetClassDefaults _output_get)))
    (Default|SetItemInfoatIndex (Variables|/Game/Blueprints/Player/BP_SCCharacter.BP_SCCharacter_C|GetActionBar1 _asbp_sccharacter) (Variables|/Game/Blueprints/Player/BP_SCCharacter.BP_SCCharacter_C|GetSelectedSlot _asbp_sccharacter) (.Item (Default|GetItemInfoatIndex (Variables|/Game/Blueprints/Player/BP_SCCharacter.BP_SCCharacter_C|GetActionBar1 _asbp_sccharacter) (Variables|/Game/Blueprints/Player/BP_SCCharacter.BP_SCCharacter_C|GetSelectedSlot _asbp_sccharacter))) (- (.Quantity (Default|GetItemInfoatIndex (Variables|/Game/Blueprints/Player/BP_SCCharacter.BP_SCCharacter_C|GetActionBar1 _asbp_sccharacter) (Variables|/Game/Blueprints/Player/BP_SCCharacter.BP_SCCharacter_C|GetSelectedSlot _asbp_sccharacter))) 1))
    (bind _output_get_2 (Variables|Default|SetSeed%20Type (.SeedType (Utilities|GetClassDefaults (.Item (Default|GetItemInfoatIndex (Variables|/Game/Blueprints/Player/BP_SCCharacter.BP_SCCharacter_C|GetActionBar1 _asbp_sccharacter) (Variables|/Game/Blueprints/Player/BP_SCCharacter.BP_SCCharacter_C|GetSelectedSlot _asbp_sccharacter)))))))
    (Variables|GrowthVariables|SetTimeBetweenStages (/ (Variables|GrowthVariables|GetTotalTimeToGrow) (Variables|GrowthVariables|GetTotalPlantStages)))
    (Variables|Default|SetIsPlanted true)
    ;[1 1 1] ThisCallsGrowPlants
    (CallFunction|SelectPlantSprites _output_get_2)
    (CallFunction|SaveFarmTileInfo)))

(event Custom|GrowPlant
  (bind _returnvalue (AddComponent|AddPaperSpriteComponent false (Math|Transform|MakeTransform (Variables|Default|GetRelativeTransformLocation) "0, 0, 0" (Variables|Default|GetRelativeScale))))
  (Rendering|Components|Sprite|SetSprite _returnvalue (Utilities|Array|Get(acopy) (Variables|Default|GetCurrentPlantMeshes) (Variables|GrowthVariables|GetCurrentPlantState)))
  (Math|Integer|IncrementInt (Variables|GrowthVariables|GetCurrentPlantState)
    (:%20%20
      (if (>= (+ (Variables|GrowthVariables|GetCurrentPlantState) 1) (Variables|GrowthVariables|GetTotalPlantStages))
        (bind _output_get (Variables|Default|SetCurrentSprite _returnvalue))
        (Rendering|Components|Sprite|SetSprite _output_get (Utilities|Array|Get(acopy) (Variables|Default|GetCurrentPlantMeshes) (- (Variables|GrowthVariables|GetTotalPlantStages) 1)))
        (Variables|Default|SetFullGrown true)
        (CallFunction|SaveFarmTileInfo)
        (else
          (CallFunction|SaveFarmTileInfo)
          (Components|DestroyComponent _returnvalue))))))

(event Custom|Harvest
  (bind _returnvalue (Transformation|GetActorLocation))
  (bind _seed (Variables|Default|GetSeed))
  (bind _relativetransformlocation (Variables|Default|GetRelativeTransformLocation))
  (bind (_totaltimetogrow _plantstages _chanceforseed _chanceforextraseed) (Utilities|GetClassDefaults _seed))
  (bind _returnvalue_2 (+ _returnvalue _relativetransformlocation))
  (bind _returnvalue_3 (+ _returnvalue_2 "3.000000,0.000000,0.000000"))
  (if (Variables|Default|GetFullGrown)
    (Components|DestroyComponent (Variables|Default|GetCurrentSprite))
    ;[1 0 0] CheckIfUsed?
    (Utilities|Casting|CastToBP_SCCharacter (Game|GetPlayerCharacter 0))
    (bind (_seed_2 _extraseed) (CallFunction|ChanceforSeed _chanceforseed _chanceforextraseed))
    (if _seed_2
      (if _extraseed
        ;[1 1 1] GiveExtraSeed(2)
        (Game|SpawnActorfromClass "/Game/Blueprints/InventorySystem/BP_MasterPickUpActor.BP_MasterPickUpActor_C" (Math|Transform|MakeTransform (+ (Transformation|GetActorLocation) (Variables|Default|GetRelativeTransformLocation) "0.000000,0.000000,10.000000") "0, 0, 0" "1.000000,1.000000,1.000000") "Undefined" "MultiplyWithRoot" 0 _seed 2 0 0)
        (else
          ;[1 1 1] GiveSeed(1)
          (Game|SpawnActorfromClass "/Game/Blueprints/InventorySystem/BP_MasterPickUpActor.BP_MasterPickUpActor_C" (Math|Transform|MakeTransform (+ (Transformation|GetActorLocation) (Variables|Default|GetRelativeTransformLocation) "0.000000,0.000000,10.000000") "0, 0, 0" "1.000000,1.000000,1.000000") "Undefined" "MultiplyWithRoot" 0 0 1 0 0))))
    (switch Utilities|FlowControl|Switch|SwitchonSeedType (Variables|Default|GetSeed%20Type)
      (:NewEnumerator1
        ;[1 1 1] logic for harvested
        (Game|SpawnActorfromClass "/Game/Blueprints/InventorySystem/BP_MasterPickUpActor.BP_MasterPickUpActor_C" (Math|Transform|MakeTransform _returnvalue_3 "0, 0, 0" "1.000000,1.000000,1.000000") "Undefined" "MultiplyWithRoot" 0 "/Game/Blueprints/InventorySystem/Items/Consumables/BP_Wheat.BP_Wheat_C" 1 0 0))
      (:NewEnumerator2
        (Game|SpawnActorfromClass "/Game/Blueprints/InventorySystem/BP_MasterPickUpActor.BP_MasterPickUpActor_C" (Math|Transform|MakeTransform _returnvalue_3 "0, 0, 0" "1.000000,1.000000,1.000000") "Undefined" "MultiplyWithRoot" 0 "/Game/Blueprints/InventorySystem/Items/Consumables/BP_Eggplant.BP_Eggplant_C" 1 0 0)))
    ;[1 1 1] ResetFarmTile
    (Variables|Default|SetFullGrown false)
    (Variables|Default|SetIsPlanted false)
    (Variables|GrowthVariables|SetCurrentPlantState 0)
    (CallFunction|SaveFarmTileInfo)))

(event Custom|SaveFarmTileInfo
  ;[1 1 1] SaveTiles
  (bind _asbp_game_instance (Utilities|Casting|CastToBP_GameInstance (Game|GetGameInstance)))
  (Utilities|Array|Add (Variables|/Game/Blueprints/BP_GameInstance.BP_GameInstance_C|GetSavedPlantStruct _asbp_game_instance) (Utilities|Struct|MakeFPlantInfo (Transformation|GetActorLocation) (Variables|Default|GetSeed%20Type) (Variables|GrowthVariables|GetCurrentPlantState)))
  (Default|SaveGame _asbp_game_instance))

(event Custom|RemoveFromSaveGame
  ;[1 1 1] SaveTiles
  (Variables|Default|SetIndexToDelete -1)
  (bind _asbp_game_instance (Utilities|Casting|CastToBP_GameInstance (Game|GetGameInstance)))
  (if (> (Utilities|Array|Length (Variables|/Game/Blueprints/BP_GameInstance.BP_GameInstance_C|GetSavedPlantStruct _asbp_game_instance)) 0)
    (for (_array_element _array_index) (Variables|/Game/Blueprints/BP_GameInstance.BP_GameInstance_C|GetSavedPlantStruct _asbp_game_instance)
      (if (Utilities|Operators|EqualEqual (.FarmTilePostion (Utilities|Struct|BreakFPlantInfo _array_element)) (Transformation|GetActorLocation) 1e+01)
        (Variables|Default|SetIndexToDelete _array_index)))
    (if (>= (Variables|Default|GetIndexToDelete) 0)
      (Utilities|Array|RemoveIndex (Variables|/Game/Blueprints/BP_GameInstance.BP_GameInstance_C|GetSavedPlantStruct _asbp_game_instance) (Variables|Default|GetIndexToDelete))
      (Default|SaveGame _asbp_game_instance))))

(event EventBeginPlay
  (bind _asbp_game_instance (Utilities|Casting|CastToBP_GameInstance (Game|GetGameInstance)))
  (EventDispatchers|BindEventtoOnDayEnded _asbp_game_instance (EventDispatchers|CreateEvent :!event Custom|GrowPlant)))

(fn ConstructionScript)

(fn SpawnfromSave
  (params (FarmTileInfo :type F%20Plant%20Info%20Structure))
  (CallFunction|SelectPlantSprites (.seedtype FarmTileInfo))
  (Variables|GrowthVariables|SetCurrentPlantState (.growthstate FarmTileInfo)))

(fn SelectPlantSprites
  (params (NewParam :type SeedType%20Enum :default "NewEnumerator0"))
  (switch Utilities|FlowControl|Switch|SwitchonSeedType NewParam
    (:NewEnumerator1
      (Variables|Default|SetCurrentPlantMeshes (.wheatmeshes (Utilities|Array|Get(acopy) (Variables|Default|GetPlantsMeshes)))))
    (:NewEnumerator2
      (Variables|Default|SetCurrentPlantMeshes (.wheatmeshes (Utilities|Array|Get(acopy) (Variables|Default|GetPlantsMeshes) 1)))))
  (CallFunction|GrowPlant)
  (return))

(fn ChanceforSeed
  (params (ChanceForSeed :type Integer) (ChanceForExtraSeed :type Integer))
  (if (== ChanceForSeed 0)
    (return false false)
    (elif (== (Math|Random|RandomIntegerinRange 1 (/ 100 ChanceForSeed)) 1)
      (if (== ChanceForExtraSeed 0)
        (if (== (Math|Random|RandomIntegerinRange 1 (/ 100 ChanceForExtraSeed)) 1)
          (return true true)
          (else
            (return true false)))
        (else
          (return true false)))
      (else
        (return false false)))))

(fn Interacted
  (params (PlayerRef :type BP%20SC%20Character%20Object%20Reference))
  (if (Variables|Default|GetIsPlanted)
    (if (Variables|Default|GetFullGrown)
      (CallFunction|Harvest))
    (else
      (CallFunction|EventPlantSeed)
      (return false))))