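; Area spawner actor for harvestable items in the inventory system, scattering random objects inside a box volume.
; On BeginPlay it loops up to NumberOfObjectsToSpawn, spawning a uniformly random class from ItemsToSpawn at a random point within the Box bounds.
; Weighted item chances and empty-space checks are noted in comments but not implemented.
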(event Custom|SpawnActorsInVolume
  (params (LastIndex :type Integer))
  (bind _box (Variables|Default|GetBox))
  (bind _itemstospawn (Variables|Default|GetItemsToSpawn))
  (for _index (range 0 LastIndex)
    ;[1 1 1] Add chance for different items
    (Game|SpawnActorfromClass (Utilities|Array|Get(acopy) _itemstospawn (Math|Random|RandomInteger (Utilities|Array|Length _itemstospawn))) (Math|Transform|MakeTransform (Math|Random|RandomPointinBoundingBox (Transformation|GetWorldLocation _box) (Components|Box|GetScaledBoxExtent _box)) "0, 0, 0" "1.000000,1.000000,1.000000") "Undefined" "MultiplyWithRoot" 0 0)))

(event EventBeginPlay
  (CallFunction|SpawnActorsinVolume (Variables|Default|GetNumberOfObjectsToSpawn)))

(fn ConstructionScript)