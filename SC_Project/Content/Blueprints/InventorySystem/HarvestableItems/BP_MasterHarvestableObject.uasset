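; Base harvestable world object that turns into a pickup item when the player interacts with it.
; Interacted calls DropItem and reports success.
; DropItem removes the object's sprite, spawns a BP_MasterPickUpActor just above it with the configured item and quantity, pops it upward with an impulse, then destroys itself.
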(event Custom|DropItem
  (Components|DestroyComponent (Variables|Default|GetObjectBaseSprite))
  (bind _returnvalue (Game|SpawnActorfromClass "/Game/Blueprints/InventorySystem/BP_MasterPickUpActor.BP_MasterPickUpActor_C" (Math|Conversions|ToTransform(Vector) (+ (Transformation|GetActorLocation) "0.000000,0.000000,10.000000")) "Undefined" "MultiplyWithRoot" 0 (Variables|DroppedItem|GetItemToDrop) (Variables|DroppedItem|GetQuantity) 0 0))
  (Physics|AddImpulse (Variables|/Game/Blueprints/InventorySystem/BP_MasterPickUpActor.BP_MasterPickUpActor_C|GetSphere _returnvalue) "0.000000,0.000000,300.000000" "None" true)
  (Actor|DestroyActor self))

(event EventBeginPlay)

(event Collision|EventActorBeginOverlap
  (params (OtherActor :type Actor%20Object%20Reference)))

(event EventTick
  (params (DeltaSeconds :type Float%20%28single-precision%29)))

(fn ConstructionScript)

(fn Interacted
  (params (PlayerRef :type BP%20SC%20Character%20Object%20Reference))
  (CallFunction|DropItem)
  (return true))