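; Inventory component that holds a fixed-size array of item class and quantity slots, persisted per container ID.
; BeginPlay loads Contents from the BP_GameInstance saved containers, then resizes it to the cell count.
; AddItem places units one at a time, filling non-full stacks before empty slots for stackable items, and returns any remainder.
; Each slot write refreshes its linked slot reference and immediately saves the game through the GameInstance.
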(event EventBeginPlay
  (bind _asbp_game_instance (Utilities|Casting|CastToBP_GameInstance (Game|GetGameInstance)))
  (Variables|Default|SetGameInstanceRef _asbp_game_instance)
  (CallFunction|LoadInventory)
  (Utilities|Array|Resize (Variables|Default|GetContents) (Variables|Default|GetCellAmmount)))

(fn SetItemInfoatIndex
  (params (Idex :type Integer) (Item :type BP%20Item%20Base%20Class%20Reference) (Quantity :type Integer))
  (bind _output_get (LocalVariables|SetLocalIndex Idex))
  (Utilities|Array|SetArrayElem (Variables|Default|GetContents) _output_get (Utilities|Struct|MakeInventoryContents Item Quantity) true)
  (Default|UpdateSLot (Utilities|Array|Get(acopy) (Variables|Default|GetSlotRef) (LocalVariables|GetLocalIndex)))
  (CallFunction|SaveInventory)
  (return))

(fn GetItemInfoatIndex
  (params (Index :type Integer))
  (LocalVariables|SetLocalIndex Index)
  (return (.item (Utilities|Array|Get(acopy) (Variables|Default|GetContents) (LocalVariables|GetLocalIndex))) (.quantity (Utilities|Array|Get(acopy) (Variables|Default|GetContents) (LocalVariables|GetLocalIndex)))))

(fn ValidateInventorySlot
  (params (Index :type Integer))
  (return (Utilities|IsValidClass (.item (Utilities|Array|Get(acopy) (Variables|Default|GetContents) Index)))))

(fn SaveInventory
  (bind (_array_element _array_index) (Utilities|Array|ForEachLoopwithBreak (Variables|/Game/Blueprints/BP_GameInstance.BP_GameInstance_C|GetSavedContainersStruct (Variables|Default|GetGameInstanceRef)) :!label _label)
    (:LoopBody
      (if (== (.ID (Utilities|Struct|BreakSaveContainersStruct _array_element)) (Variables|Default|GetID))
        (goto _label Break)))
    (:Completed
      (if (== (.ID (Utilities|Struct|BreakSaveContainersStruct _array_element)) (Variables|Default|GetID))
        (Utilities|Array|SetArrayElem (Variables|/Game/Blueprints/BP_GameInstance.BP_GameInstance_C|GetSavedContainersStruct (Variables|Default|GetGameInstanceRef)) _array_index (Utilities|Struct|MakeSaveContainersStruct (Variables|Default|GetID) (Variables|Default|GetContents)) true)
        (Development|PrintString (Utilities|String|Append "found save game container, updated on id: " (Utilities|String|ToString(Integer) (Variables|Default|GetID))) true true "(R=0.000000,G=0.660000,B=1.000000,A=1.000000)" 5.0)
        (Default|SaveGame (Variables|Default|GetGameInstanceRef))
        (return)
        (else
          (Utilities|Array|Add (Variables|/Game/Blueprints/BP_GameInstance.BP_GameInstance_C|GetSavedContainersStruct (Variables|Default|GetGameInstanceRef)) (Utilities|Struct|MakeSaveContainersStruct (Variables|Default|GetID) (Variables|Default|GetContents)))
          (Development|PrintString (Utilities|String|Append "Didnt find save game container, added with id: " (Utilities|String|ToString(Integer) (Variables|Default|GetID))) true true "(R=0.000000,G=0.660000,B=1.000000,A=1.000000)" 5.0)
          (Default|SaveGame (Variables|Default|GetGameInstanceRef))
          (return))))))

(fn LoadInventory
  (Development|PrintString "Trying to load" true true "(R=1.000000,G=0.000000,B=0.111448,A=1.000000)")
  (bind (_array_element _array_index) (Utilities|Array|ForEachLoopwithBreak (Variables|/Game/Blueprints/BP_GameInstance.BP_GameInstance_C|GetSavedContainersStruct (Variables|Default|GetGameInstanceRef)) :!label _label)
    (:LoopBody
      (if (== (.ID (Utilities|Struct|BreakSaveContainersStruct _array_element)) (Variables|Default|GetID))
        (goto _label Break)))
    (:Completed
      (if (== (.ID (Utilities|Struct|BreakSaveContainersStruct _array_element)) (Variables|Default|GetID))
        (Variables|Default|SetID (.id (Utilities|Array|Get(acopy) (Variables|/Game/Blueprints/BP_GameInstance.BP_GameInstance_C|GetSavedContainersStruct (Variables|Default|GetGameInstanceRef)) _array_index)))
        (Variables|Default|SetContents (.contents (Utilities|Array|Get(acopy) (Variables|/Game/Blueprints/BP_GameInstance.BP_GameInstance_C|GetSavedContainersStruct (Variables|Default|GetGameInstanceRef)) _array_index)))
        (return)
        (else
          (return))))))

(fn AddItem
  (params (ItemToAdd :type BP%20Item%20Base%20Class%20Reference) (QuantityToAdd :type Integer))
  (bind (_isvalid _slotindex) (CallFunction|SearchValidEmptySlot))
  (bind (_valid _index) (CallFunction|ValidStackableIndex))
  (bind (_isvalid_2 _slotindex_2) (CallFunction|SearchValidEmptySlot))
  (Variables|Default|SetItem%20to%20Add ItemToAdd)
  (Variables|Default|SetQuantity%20to%20Add QuantityToAdd)
  (if (.stackable (Utilities|GetClassDefaults (Variables|Default|GetItem%20to%20Add))) :!label _label
    (if _valid
      (CallFunction|AddOnetoStackatIndex _index)
      (if (> (Variables|Default|GetQuantity%20to%20Add) 0)
        (goto _label)
        (else
          (return true 0)))
      (elif _isvalid_2
        (CallFunction|AddOneatIndex _slotindex_2)
        (if (> (Variables|Default|GetQuantity%20to%20Add) 0)
          (goto _label)
          (else
            (return true 0)))
        (else
          (return false (Variables|Default|GetQuantity%20to%20Add)))))
    (else
      ;[0.3021 0.3021 0.3021] NonStackableItems
      (if _isvalid :!label _label_2
        (CallFunction|AddOneatIndex _slotindex)
        (if (> (Variables|Default|GetQuantity%20to%20Add) 0)
          (goto _label_2)
          (else
            (return true 0)))
        (else
          (return false (Variables|Default|GetQuantity%20to%20Add)))))))

(fn SearchValidEmptySlot
  (bind (_array_element _array_index) (Utilities|Array|ForEachLoopwithBreak (Variables|Default|GetContents) :!label _label)
    (:LoopBody
      (if (not (Utilities|IsValidClass (.Item (Utilities|Struct|BreakInventoryContents _array_element))))
        (goto _label Break)))
    (:Completed
      (if (not (Utilities|IsValidClass (.Item (Utilities|Struct|BreakInventoryContents _array_element))))
        (return true _array_index)
        (else
          (return false 0))))))

(fn AddOneatIndex
  (params (Index :type Integer))
  (bind _output_get (LocalVariables|SetLocalIndex Index))
  (Utilities|Array|SetArrayElem (Variables|Default|GetContents) _output_get (Utilities|Struct|MakeInventoryContents (Variables|Default|GetItem%20to%20Add) 1) true)
  (Default|UpdateSlot (Utilities|Array|Get(acopy) (Variables|Default|GetSlotRef) (LocalVariables|GetLocalIndex)))
  (CallFunction|SaveInventory)
  (bind _result (Math|Integer|DecrementInt (Variables|Default|GetQuantity%20to%20Add))
    (:%20%20
      (Variables|Default|SetQuantity%20to%20Add _result)
      (return))))

(fn ValidStackableIndex
  (bind _item_to_add (Variables|Default|GetItem%20to%20Add))
  (bind (_array_element _array_index) (Utilities|Array|ForEachLoopwithBreak (Variables|Default|GetContents) :!label _label)
    (:LoopBody
      (if (and (== (.Item (Utilities|Struct|BreakInventoryContents _array_element)) _item_to_add) (< (.Quantity (Utilities|Struct|BreakInventoryContents _array_element)) (.maxstacksize (Utilities|GetClassDefaults _item_to_add))))
        (goto _label Break)))
    (:Completed
      (if (and (== (.Item (Utilities|Struct|BreakInventoryContents _array_element)) _item_to_add) (< (.Quantity (Utilities|Struct|BreakInventoryContents _array_element)) (.maxstacksize (Utilities|GetClassDefaults _item_to_add))))
        (return true _array_index)
        (else
          (return false 0))))))

(fn AddOnetoStackatIndex
  (params (Index :type Integer))
  (bind _output_get (LocalVariables|SetLocalIndex Index))
  (Utilities|Array|SetArrayElem (Variables|Default|GetContents) _output_get (Utilities|Struct|MakeInventoryContents (Variables|Default|GetItem%20to%20Add) (+ (.quantity (Utilities|Array|Get(acopy) (Variables|Default|GetContents) (LocalVariables|GetLocalIndex))) 1)))
  (Default|UpdateSlot (Utilities|Array|Get(acopy) (Variables|Default|GetSlotRef) (LocalVariables|GetLocalIndex)))
  (CallFunction|SaveInventory)
  (Variables|Default|SetQuantity%20to%20Add (- (Variables|Default|GetQuantity%20to%20Add) 1))
  (return))