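; BP_MasterStorage is a storage actor in the inventory system, by its name the base for storage objects, that the player interacts with to view its contents.
; Interacted passes its InventoryComponent to the player HUD's PlayerInventory widget to generate the storage inventory, then switches that widget to its second page.
; The function always returns false, and the event graph and construction script are empty.
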(event EventBeginPlay)

(event Collision|EventActorBeginOverlap
  (params (OtherActor :type Actor%20Object%20Reference)))

(event EventTick
  (params (DeltaSeconds :type Float%20%28single-precision%29)))

(fn ConstructionScript)

(fn Interacted
  (params (PlayerRef :type BP%20SC%20Character%20Object%20Reference))
  (Variables|Default|SetPlayer%20Ref PlayerRef)
  (Default|GenerateStorageInventory (Variables|/Game/Blueprints/WBP_HUD.WBP_HUD_C|GetPlayerInventory (Variables|/Game/Blueprints/Player/BP_SCCharacter.BP_SCCharacter_C|GetHudRef (Variables|Default|GetPlayer%20Ref))) (Variables|Default|GetInventoryComponent))
  (Variables|/Script/UMG.WidgetSwitcher|SetActiveWidgetIndex (Variables|/Game/Blueprints/InventorySystem/Interface/WBP_Inventroy.WBP_Inventroy_C|GetWidgetSwitcher_131 (Variables|/Game/Blueprints/WBP_HUD.WBP_HUD_C|GetPlayerInventory (Variables|/Game/Blueprints/Player/BP_SCCharacter.BP_SCCharacter_C|GetHudRef (Variables|Default|GetPlayer%20Ref)))) 1)
  (return false))