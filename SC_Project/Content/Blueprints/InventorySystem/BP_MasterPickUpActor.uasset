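; Base pickup actor for the inventory system that hands an item and quantity to an overlapping BP_SCCharacter.
; On BeginPlay it sets its Paper2D sprite from the item class defaults and fills its pop-up info widget.
; On sphere overlap it tries the action bar first, then sends any remainder to the inventory component.
; It destroys itself on success, otherwise keeps the leftover quantity and refreshes the pop-up.
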(event OnComponentBeginOverlap(Sphere)
  (params (OverlappedComponent :type Primitive%20Component%20Object%20Reference) (OtherActor :type Actor%20Object%20Reference) (OtherComp :type Primitive%20Component%20Object%20Reference) (OtherBodyIndex :type Integer) (bFromSweep :type Boolean) (SweepResult :type Hit%20Result%20Structure%20%28by%20ref%29))
  (bind _asbp_sccharacter (Utilities|Casting|CastToBP_SCCharacter OtherActor))
  (bind (_success _remainder) (Default|AddItem (Variables|/Game/Blueprints/Player/BP_SCCharacter.BP_SCCharacter_C|GetActionBar1 _asbp_sccharacter) (Variables|Default|GetItem) (Variables|Default|GetQuantity)))
  (if _success
    (Actor|DestroyActor)
    (else
      (bind (_success_2 _remainder_2) (Default|AddItem (Variables|/Game/Blueprints/Player/BP_SCCharacter.BP_SCCharacter_C|GetInventoryComponent _asbp_sccharacter) (Variables|Default|GetItem) _remainder))
      (if _success_2
        (Actor|DestroyActor)
        (else
          (bind _output_get (Variables|Default|SetQuantity _remainder_2))
          (Default|UpdateInfo (Variables|Default|GetAs%20WBP%20Pop%20Up%20Info) (Variables|Default|GetItem) _output_get))))))

(event EventBeginPlay
  (bind _aswbp_pop_up_info (Utilities|Casting|CastToWBP_PopUpInfo (UserInterface|GetWidget (Variables|Default|GetPupUpInfo))))
  (bind _output_get (Variables|Default|SetAs%20WBP%20Pop%20Up%20Info _aswbp_pop_up_info))
  (Default|UpdateInfo _output_get (Variables|Default|GetItem) (Variables|Default|GetQuantity))
  (Physics|AddImpulse (Variables|Default|GetSphere) "0, 0, 0" "None" true)
  (Rendering|Components|Sprite|SetSprite (Variables|Default|GetPaperSprite) (.sprite (.ItemInfo (Utilities|GetClassDefaults (Variables|Default|GetItem))))))

(event Collision|EventActorBeginOverlap
  (params (OtherActor :type Actor%20Object%20Reference)))

(event EventTick
  (params (DeltaSeconds :type Float%20%28single-precision%29)))

(fn ConstructionScript)