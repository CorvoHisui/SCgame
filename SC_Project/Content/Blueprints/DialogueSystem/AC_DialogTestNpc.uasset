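; Dialogue component for a test NPC, overriding Dialog to define a small branching conversation with emotion reactions.
; A switch on DialogTreeIndex selects the tree, and each AddDialog returns Updated to play emotions or Pass Through to advance or close.
; The friendly reply saves index 1, giving a random friendly greeting in later talks.
; The rude reply progresses the "Bad Neighbour" achievement and leaves the index unchanged.
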(event EventBeginPlay)

(event EventTick
  (params (DeltaSeconds :type Float%20%28single-precision%29)))

(fn Dialog
  (|CallParentFunction)
  (switch int (Variables|Default|GetDialogTreeIndex)
    (:0
      (bind (_state _optionindex) (CallFunction|AddDialog "TestNpc" "Hello, I am indeed talking to you" (Utilities|Array|MakeArray "Pleasure to meet you" "Do you want a medal?")))
      (switch Utilities|FlowControl|Switch|SwitchonEnumDialogValue _state
        (:NewEnumerator0
          (switch int _optionindex
            (:0
              ;[1 0 0] No switch on int when only one option
              (bind _state_2 (CallFunction|AddDialog "TestNpc" "And the same to you!!" (Utilities|Array|MakeArray "Have a good day!!")))
              (switch Utilities|FlowControl|Switch|SwitchonEnumDialogValue _state_2
                (:NewEnumerator0
                  (Default|HideEmotion (Variables|Default|GetOwnerNPC))
                  (CallFunction|SetDialogTreeIndex 1)
                  (CallFunction|ClearDialogProgress)
                  (CallFunction|CloseConversation))
                (:NewEnumerator1
                  (Default|PlayEmotion (Variables|Default|GetOwnerNPC) true "NewEnumerator3"))))
            (:1
              (bind _state_3 (CallFunction|AddDialog "TestNpc" "Well fuck you, annoying shit" (Utilities|Array|MakeArray "Fuck you, Bye")))
              (switch Utilities|FlowControl|Switch|SwitchonEnumDialogValue _state_3
                (:NewEnumerator0
                  (Default|HideEmotion (Variables|Default|GetOwnerNPC))
                  (CallFunction|ClearDialogProgress)
                  (CallFunction|CloseConversation))
                (:NewEnumerator1
                  (CallFunction|UnlockAchievement "Bad Neighbour" 1)
                  (Default|PlayEmotion (Variables|Default|GetOwnerNPC) true "NewEnumerator2"))))))
        (:NewEnumerator1)))
    (:1
      (bind _state_4 (CallFunction|AddDialog "TestNpc" (Utilities|Select :Index (Math|Random|RandomIntegerinRange 0 1) :Option%200 "You are so Nice!!" :Option%201 "*What a nice person* 
Have a lovely day!") (Utilities|Array|MakeArray "Thank you!!")))
      (switch Utilities|FlowControl|Switch|SwitchonEnumDialogValue _state_4
        (:NewEnumerator0
          (Default|HideEmotion (Variables|Default|GetOwnerNPC))
          (CallFunction|RemoveDialogProgress 1)
          (CallFunction|CloseConversation))
        (:NewEnumerator1
          (Default|PlayEmotion (Variables|Default|GetOwnerNPC) false "NewEnumerator10"))))))