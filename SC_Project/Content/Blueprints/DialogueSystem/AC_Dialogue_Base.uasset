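; Base dialogue component for NPCs that runs branching conversations through a WB_Dialog widget and handles quest item hand-ins.
; Each choice is saved by step index, then the empty Dialog function, meant for overriding, replays from the start.
; AddDialog returns saved choices and displays steps lacking one.
; HandInQuest deducts a sufficient stack from the interacting player's inventory; its action bar search is disconnected.
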(fn OpenConversation
  (bind _returnvalue (UserInterface|CreateWidget "/Game/Blueprints/DialogueSystem/UI/WB_Dialog.WB_Dialog_C" 0 self))
  (bind _output_get (Variables|Default|SetDialogWidget _returnvalue))
  (UserInterface|Viewport|AddtoViewport _output_get 0)
  (bind _asbp_test_npc (Utilities|Casting|CastToBP_TestNpc (Components|GetOwner)))
  (Variables|Default|SetOwnerNPC _asbp_test_npc)
  (CallFunction|ProgressDialog))

(fn CloseConversation
  (Widget|RemovefromParent (Variables|Default|GetDialogWidget))
  (Class|BPIInteractable|ConversationClosed(Message) (Components|GetOwner)))

(fn ProgressDialog
  (Variables|Default|SetDialogIndex -1)
  (CallFunction|Dialog))

(fn Dialog)

(fn AddDialog
  (params (SpeakerName :type Text) (DialogueText :type Text) (OptionsText :type Array%20of%20Texts))
  (bind _dialogprogress (Variables|Default|GetDialogProgress))
  (bind _dialogindex (Variables|Default|GetDialogIndex))
  (bind (_value _returnvalue) (Utilities|Map|Find _dialogprogress _dialogindex))
  (Math|Integer|IncrementInt (Variables|Default|GetDialogIndex)
    (:%20%20
      (if _returnvalue
        (return "NewEnumerator0" _value)
        (else
          (Default|UpdateDialogText (Variables|Default|GetDialogWidget) (Variables|Default|GetDialogIndex) SpeakerName DialogueText OptionsText)
          (return "NewEnumerator1" 0))))))

(fn UpdateSelectedOption
  (params (ProgressIndex :type Integer%20%28by%20ref%29) (OptionIndex :type Integer%20%28by%20ref%29))
  (Utilities|Map|Add (Variables|Default|GetDialogProgress) ProgressIndex OptionIndex)
  (CallFunction|ProgressDialog))

(fn ClearDialogProgress
  (Utilities|Map|Clear (Variables|Default|GetDialogProgress)))

(fn RemoveDialogProgress
  (params (ProgresSteps :type Integer))
  (for _index (range 0 ProgresSteps)
    (Utilities|Map|Remove (Variables|Default|GetDialogProgress) (- (Variables|Default|GetDialogIndex) _index))))

(fn SetDialogTreeIndex
  (params (DialogTreeIndex :type Integer))
  (Variables|Default|SetDialogTreeIndex DialogTreeIndex))

(fn HandinQuest
  (params (NewParam :type BP%20Item%20Base%20Class%20Reference) (Quantity :type Integer))
  (Variables|Quest|SetItemToHand NewParam)
  (Variables|Quest|SetQuantityToHand Quantity)
  (bind _asbp_sccharacter (Utilities|Casting|CastToBP_SCCharacter (Variables|/Game/Blueprints/DialogueSystem/NPC/BP_TestNpc.BP_TestNpc_C|GetInteractInstigator (Variables|Default|GetOwnerNPC))))
  ;[0.1765 0.5238 1 0.75] SearchMainInventory
  ;;[1 1 1] SearchForItemOnInventory
  (bind _array_index (Utilities|Array|ForEachLoopwithBreak (Variables|/Game/Blueprints/InventorySystem/InventoryComponent.InventoryComponent_C|GetSlotRef (Variables|/Game/Blueprints/Player/BP_SCCharacter.BP_SCCharacter_C|GetInventoryComponent _asbp_sccharacter)) :!label _label)
    (:LoopBody
      (if (and (== (Variables|Quest|GetItemToHand) (.Item (Default|GetItemInfoatIndex (Variables|/Game/Blueprints/Player/BP_SCCharacter.BP_SCCharacter_C|GetInventoryComponent _asbp_sccharacter) _array_index))) (>= (.Quantity (Default|GetItemInfoatIndex (Variables|/Game/Blueprints/Player/BP_SCCharacter.BP_SCCharacter_C|GetInventoryComponent _asbp_sccharacter) _array_index)) (Variables|Quest|GetQuantityToHand)))
        (Variables|Quest|SetItemFound true)
        (Variables|Quest|SetIndexOfItemFound _array_index)
        (goto _label Break)))
    (:Completed
      (if (Variables|Quest|GetItemFound)
        (if (== (- (.Quantity (Default|GetItemInfoatIndex (Variables|/Game/Blueprints/Player/BP_SCCharacter.BP_SCCharacter_C|GetInventoryComponent _asbp_sccharacter) (Variables|Quest|GetIndexOfItemFound))) (Variables|Quest|GetQuantityToHand)) 0)
          (Default|SetItemInfoatIndex (Variables|/Game/Blueprints/Player/BP_SCCharacter.BP_SCCharacter_C|GetInventoryComponent _asbp_sccharacter) (Variables|Quest|GetIndexOfItemFound))
          (return true)
          (else
            (Default|SetItemInfoatIndex (Variables|/Game/Blueprints/Player/BP_SCCharacter.BP_SCCharacter_C|GetInventoryComponent _asbp_sccharacter) (Variables|Quest|GetIndexOfItemFound) (Variables|Quest|GetItemToHand) (- (.Quantity (Default|GetItemInfoatIndex (Variables|/Game/Blueprints/Player/BP_SCCharacter.BP_SCCharacter_C|GetInventoryComponent _asbp_sccharacter) (Variables|Quest|GetIndexOfItemFound))) (Variables|Quest|GetQuantityToHand)))
            (return true)))
        (else
          (return false))))))