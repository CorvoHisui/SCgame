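; BP_GridSetUp is a grid setup Blueprint that builds a flat grid of static mesh components at BeginPlay.
; Nested loops over GridX and GridY add one component per cell, spaced by GridSize in the actor's local XY plane.
; Both axes are offset by half the GridX extent, so the grid is centred on the actor only when GridY equals GridX.
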(event EventBeginPlay
  (bind _gridx (Variables|Default|GetGridX))
  (bind _gridsize (Variables|Default|GetGridSize))
  (bind _returnvalue (- _gridx 1))
  (bind _returnvalue_2 (* _gridsize _returnvalue))
  (bind _returnvalue_3 (/ _returnvalue_2 2))
  (for _index (range 0 (- (Variables|Default|GetGridX) 1))
    (for _index_2 (range 0 (- (Variables|Default|GetGridY) 1))
      (AddComponent|AddStaticMeshComponent false (Math|Transform|MakeTransform (Math|Vector|MakeVector (Math|Conversions|ToFloat(Integer) (- (- (* _index _gridsize) _returnvalue_3) 0)) (Math|Conversions|ToFloat(Integer) (- (- (* _index_2 _gridsize) _returnvalue_3) 0)) 0.0))))))

(fn ConstructionScript)