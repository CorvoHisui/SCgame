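; Player character with left/right facing, animation-node jumps for airborne and landing, and a grid-based block building mode.
; Q toggles a BP_GridSetUp snapped to the player's position, which Tick re-centers as the player moves away.
; Each tick, a mouse-ray trace highlights the hovered cell through material opacity.
; Left click traces down onto that cell to destroy an existing BP_TestBlock or spawn one if empty.
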(event Custom|CenterGrid
  (bind _returnvalue (Transformation|GetActorLocation))
  (bind _divisor (Variables|Default|GetDivisor))
  ;[1 1 1] Update Grid To Player Positon
  (Utilities|IsValid (Variables|Default|GetGridSetUp)
    (:Is%20Valid
      (bind _output_get (Variables|Default|SetGridSpawnPoint (Math|Vector|MakeVector (* (.ReturnValue (Math|Float|Division(WholeandRemainder) (.x _returnvalue) _divisor)) _divisor) (* (.ReturnValue (Math|Float|Division(WholeandRemainder) (.y _returnvalue) _divisor)) _divisor) (- (.z _returnvalue) 44.0))))
      (Transformation|SetActorLocation (Variables|Default|GetGridSetUp) _output_get false false))))

(event EventBeginPlay)

(event Collision|EventActorBeginOverlap
  (params (OtherActor :type Actor%20Object%20Reference)))

(event EventTick
  (params (DeltaSeconds :type Float%20%28single-precision%29))
  (bind _returnvalue (Game|GetPlayerController 0))
  (bind (_worldlocation _worlddirection) (Game|Player|ConvertMouseLocationToWorldSpace _returnvalue))
  (|CallParentFunction DeltaSeconds)
  (Utilities|FlowControl|Sequence
    (:then_0
      (CallFunction|RotateCharacter))
    (:then_1
      (Utilities|IsValid (Variables|Default|GetGridSetUp)
        (:Is%20Valid
          (if (> (Math|Vector|VectorLength (- (- (Transformation|GetActorLocation) "0.000000,0.000000,-46.000000") (Variables|Default|GetGridSpawnPoint))) 5e+01)
            (CallFunction|CenterGrid)))))
    (:then_2
      ;[1 1 1] Show / Hide Grid Cells
      (bind (_outhit _returnvalue_2) (Collision|LineTraceForObjects _worldlocation (+ _worldlocation (* _worlddirection 1e+03)) (Utilities|Array|MakeArray "ObjectTypeQuery7") false 0 "None"))
      (if _returnvalue_2
        (Utilities|IsValid (.hitcomponent _outhit) ; Conect from this truee to range in grid
          (:Is%20Valid
            (bind _asstatic_mesh_component (Utilities|Casting|CastToStaticMeshComponent (.hitcomponent _outhit))
              (:then
                (CallFunction|MakePreviousCellInvisible)
                (bind _output_get (Variables|Default|SetSelectedGridCell _asstatic_mesh_component))
                (Rendering|Material|SetScalarParameterValueonMaterials _output_get "Opacity" 0.66))
              (:CastFailed
                (CallFunction|MakePreviousCellInvisible))))
          (:Is%20Not%20Valid
            (CallFunction|MakePreviousCellInvisible)))
        (else
          (CallFunction|MakePreviousCellInvisible))))))

(event EventOnLanded
  (params (Hit :type Hit%20Result%20Structure%20%28by%20ref%29))
  (Class|PaperZDAnimInstance|JumptoNode (Variables|/Script/PaperZD.PaperZDAnimationComponent|GetAnimInstance (Variables|Default|GetAnimationComponent)) "Landed" "None"))

(event Input|ActionEvents|InputActionJump
  (params (Key :type Key%20Structure :default "None"))
  (:Pressed
    (Components|Movement|StopMovementImmediately (Variables|Character|GetCharacterMovement))
    (Variables|Default|SetIsMovementLocked false)
    (Class|PaperZDAnimInstance|JumptoNode (Variables|/Script/PaperZD.PaperZDAnimationComponent|GetAnimInstance (Variables|Default|GetAnimationComponent)) "airborne" "None"))
  (:Released
    (Character|StopJumping)))

(event Input|AxisEvents|InputAxisFoward
  (params (AxisValue :type Float%20%28single-precision%29))
  (if (not (Variables|Default|GetIsMovementLocked))
    (Pawn|Input|AddMovementInput "1.000000,0.000000,0.000000" AxisValue false)))

(event Input|AxisEvents|InputAxisMoveUp
  (params (AxisValue :type Float%20%28single-precision%29))
  (if (not (Variables|Default|GetIsMovementLocked))
    (Pawn|Input|AddMovementInput "0.000000,-1.000000,0.000000" AxisValue false)))

(event Input|MouseEvents|LeftMouseButton
  (params (Key :type Key%20Structure :default "None"))
  (bind _selectedgridcell (Variables|Default|GetSelectedGridCell))
  (bind _returnvalue (Transformation|GetWorldLocation _selectedgridcell))
  (:Pressed
    (Utilities|IsValid (Variables|Default|GetGridSetUp)
      (:Is%20Valid
        (Utilities|IsValid (Variables|Default|GetSelectedGridCell)
          (:Is%20Valid
            (bind (_outhit _returnvalue_2) (Collision|LineTraceForObjects (+ _returnvalue "0.000000,0.000000,64.000000") _returnvalue (Utilities|Array|MakeArray "ObjectTypeQuery2" "ObjectTypeQuery2") false 0 "ForDuration"))
            (if _returnvalue_2
              (bind _asbp_test_block (Utilities|Casting|CastToBP_TestBlock (.HitActor (Collision|BreakHitResult _outhit))))
              (Actor|DestroyActor _asbp_test_block) ; if actor already exist
              (else
                (Game|SpawnActorfromClass "/Game/Assets/Grid/BP_TestBlock.BP_TestBlock_C" (Math|Transform|MakeTransform _returnvalue) "Undefined" "MultiplyWithRoot" 0 0) ; If grid empty, spawn actor
              ))))))))

(event Input|KeyboardEvents|Q
  (params (Key :type Key%20Structure :default "None"))
  (bind _returnvalue (Transformation|GetActorLocation))
  (bind _divisor (Variables|Default|GetDivisor))
  (:Pressed
    (Utilities|IsValid (Variables|Default|GetGridSetUp)
      (:Is%20Valid
        (Actor|DestroyActor (Variables|Default|GetGridSetUp))
        (Variables|Default|SetGridSetUp 0))
      (:Is%20Not%20Valid
        ;[1 1 1] Spawn Grid At Player Position
        (bind _output_get (Variables|Default|SetGridSpawnPoint (Math|Vector|MakeVector (* (.ReturnValue (Math|Float|Division(WholeandRemainder) (.x _returnvalue) _divisor)) _divisor) (* (.ReturnValue (Math|Float|Division(WholeandRemainder) (.y _returnvalue) _divisor)) _divisor) (- (.z _returnvalue) 44.0))))
        (bind _returnvalue_2 (Game|SpawnActorfromClass "/Game/Blueprints/Grid/BP_GridSetUp.BP_GridSetUp_C" (Math|Transform|MakeTransform _output_get) "Undefined" "MultiplyWithRoot" 0 0))
        (Variables|Default|SetGridSetUp _returnvalue_2)))))

(fn ConstructionScript)

(fn MakePreviousCellInvisible
  (bind _selectedgridcell (Variables|Default|GetSelectedGridCell))
  (Utilities|IsValid _selectedgridcell
    (:Is%20Valid
      (Rendering|Material|SetScalarParameterValueonMaterials _selectedgridcell "Opacity" 0.33))))

(fn RotateCharacter
  (bind _returnvalue (Pawn|GetController))
  (bind _returnvalue_2 (Pawn|GetController))
  (Math|Float|CompareFloat (.X (Math|Vector|BreakVector (Variables|/Script/Engine.MovementComponent|GetVelocity (Pawn|GetMovementComponent)))) 0.0
    (:>
      ;[0 0.4745 1] Look Right
      (Utilities|IsValid _returnvalue_2
        (:Is%20Valid
          (Pawn|SetControlRotation _returnvalue_2 (Math|Rotator|MakeRotator 0.0 0.0 0.0)))))
    (:<
      ;[0 0.4745 1] Look Left
      (Utilities|IsValid _returnvalue
        (:Is%20Valid
          (Pawn|SetControlRotation _returnvalue (Math|Rotator|MakeRotator 0.0 0.0 1.8e+02)))))))