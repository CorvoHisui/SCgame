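; Player character handling hotbar, inventory and escape menus, item use and farm grid placement.
; Shoulder, wheel and key input select a hotbar slot, updating the held mesh.
; Interact falls through to timed consumption, repeating while E is held, or equipping, implemented only for headgear.
; Tick traces under the mouse to highlight cells by material opacity; clicking spawns farm tiles or removes test blocks; key 1 fills test inventory.
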(event Custom|ConsumeItem
  (bind _actionbar1 (Variables|Default|GetActionBar1))
  (bind _selectedslot (Variables|Default|GetSelectedSlot))
  (bind (_item _quantity) (Default|GetItemInfoatIndex _actionbar1 _selectedslot))
  (bind _asbp_consumable_base (Utilities|Casting|CastToBP_ConsumableBaseClass (.Item (Default|GetItemInfoatIndex (Variables|Default|GetActionBar1) (Variables|Default|GetSelectedSlot)))))
  (Utilities|FlowControl|Delay (.Timer (Utilities|GetClassDefaults _asbp_consumable_base)))
  (if (Variables|Default|GetInteractKey)
    ;[1 0 0] CHANGE THIS AT SOME POINT
    (bind _returnvalue (Game|SpawnActorfromClass _asbp_consumable_base (Math|Transform|MakeTransform "0.000000,0.000000,-500.000000" "0, 0, 0" "1.000000,1.000000,1.000000") "Undefined" "MultiplyWithRoot" 0 0))
    (Default|ApplyEffect _returnvalue)
    (Actor|DestroyActor _returnvalue)
    (Default|SetItemInfoatIndex (Variables|Default|GetActionBar1) (Variables|Default|GetSelectedSlot) _item (- _quantity 1))
    (CallFunction|HoldItem)
    (Default|SaveGame (Variables|/Game/Blueprints/UI/Overlay/WBP_InventoryOverlay.WBP_InventoryOverlay_C|GetGameInstanceRef (Variables|Default|GetHudRef)))
    (CallFunction|ConsumeItem)))

(event Input|EnhancedActionEvents|EnhancedInputActionIA_ToggleEscapeMenu
  (params (ActionValue :type Boolean) (ElapsedSeconds :type Float%20%28double-precision%29) (TriggeredSeconds :type Float%20%28double-precision%29) (InputAction :type Input%20Action%20Object%20Reference :default "/Game/Blueprints/Input/InputActions/IA_ToggleEscapeMenu.IA_ToggleEscapeMenu"))
  (:Started
    (CallFunction|ToggleEscapeMenu)))

(event Input|EnhancedActionEvents|EnhancedInputActionIA_ControllerConfirm
  (params (ActionValue :type Boolean) (ElapsedSeconds :type Float%20%28double-precision%29) (TriggeredSeconds :type Float%20%28double-precision%29) (InputAction :type Input%20Action%20Object%20Reference :default "/Game/Blueprints/Input/InputActions/ControllerExclusive/IA_ControllerConfirm.IA_ControllerConfirm"))
  (bind _hudref (Variables|Default|GetHudRef))
  (bind _focusedslot (Variables|/Game/Blueprints/UI/Overlay/WBP_InventoryOverlay.WBP_InventoryOverlay_C|GetFocusedSlot _hudref))
  (if (Utilities|IsValid _focusedslot)
    (Default|Click _focusedslot false)))

(event Input|EnhancedActionEvents|EnhancedInputActionIA_ControllerDropItem
  (params (ActionValue :type Boolean) (ElapsedSeconds :type Float%20%28double-precision%29) (TriggeredSeconds :type Float%20%28double-precision%29) (InputAction :type Input%20Action%20Object%20Reference :default "/Game/Blueprints/Input/InputActions/ControllerExclusive/IA_ControllerDropItem.IA_ControllerDropItem"))
  (bind _hudref (Variables|Default|GetHudRef))
  (bind _wbp_puckup (Variables|/Game/Blueprints/UI/Overlay/WBP_InventoryOverlay.WBP_InventoryOverlay_C|GetWBP_PuckUp _hudref))
  (if (Default|Validate _wbp_puckup)
    (CallFunction|DropItem (Variables|/Game/Blueprints/InventorySystem/Interface/WBP_PuckUp.WBP_PuckUp_C|GetItem _wbp_puckup) (Variables|/Game/Blueprints/InventorySystem/Interface/WBP_PuckUp.WBP_PuckUp_C|GetQuantity _wbp_puckup))
    (Default|UpdateInfo _wbp_puckup)))

(event Input|EnhancedActionEvents|EnhancedInputActionIA_ControllerRighthoulder
  (params (ActionValue :type Boolean) (ElapsedSeconds :type Float%20%28double-precision%29) (TriggeredSeconds :type Float%20%28double-precision%29) (InputAction :type Input%20Action%20Object%20Reference :default "/Game/Blueprints/Input/InputActions/ControllerExclusive/IA_ControllerRighthoulder.IA_ControllerRighthoulder"))
  ;[1 1 1] HotbarNavigation
  (:Started
    (Utilities|FlowControl|Sequence
      (:then_0
        (Variables|Default|SetSelectedSlot (+ (Variables|Default|GetSelectedSlot) 1))
        (if (> (Variables|Default|GetSelectedSlot) (- (Variables|/Game/Blueprints/InventorySystem/InventoryComponent.InventoryComponent_C|GetColumns (Variables|Default|GetActionBar1)) 1))
          (Variables|Default|SetSelectedSlot 0)
          (elif (< (Variables|Default|GetSelectedSlot) 0)
            (Variables|Default|SetSelectedSlot (- (Variables|/Game/Blueprints/InventorySystem/InventoryComponent.InventoryComponent_C|GetColumns (Variables|Default|GetActionBar1)) 1)))))
      (:then_1
        (CallFunction|UpdateSelectedSlot)))))

(event Input|EnhancedActionEvents|EnhancedInputActionIA_ControllerLeftShoulder
  (params (ActionValue :type Boolean) (ElapsedSeconds :type Float%20%28double-precision%29) (TriggeredSeconds :type Float%20%28double-precision%29) (InputAction :type Input%20Action%20Object%20Reference :default "/Game/Blueprints/Input/InputActions/ControllerExclusive/IA_ControllerLeftShoulder.IA_ControllerLeftShoulder"))
  ;[1 1 1] HotbarNavigation
  (:Started
    (Utilities|FlowControl|Sequence
      (:then_0
        (Variables|Default|SetSelectedSlot (- (Variables|Default|GetSelectedSlot) 1))
        (if (> (Variables|Default|GetSelectedSlot) (- (Variables|/Game/Blueprints/InventorySystem/InventoryComponent.InventoryComponent_C|GetColumns (Variables|Default|GetActionBar1)) 1))
          (Variables|Default|SetSelectedSlot 0)
          (elif (< (Variables|Default|GetSelectedSlot) 0)
            (Variables|Default|SetSelectedSlot (- (Variables|/Game/Blueprints/InventorySystem/InventoryComponent.InventoryComponent_C|GetColumns (Variables|Default|GetActionBar1)) 1)))))
      (:then_1
        (CallFunction|UpdateSelectedSlot)))))

(event Input|EnhancedActionEvents|EnhancedInputActionIA_MouseWheel
  (params (ActionValue :type Float%20%28double-precision%29) (ElapsedSeconds :type Float%20%28double-precision%29) (TriggeredSeconds :type Float%20%28double-precision%29) (InputAction :type Input%20Action%20Object%20Reference :default "/Game/Blueprints/Input/InputActions/IA_MouseWheel.IA_MouseWheel"))
  ;[1 1 1] HotbarNavigation
  (Utilities|FlowControl|Sequence
    (:then_0
      (Variables|Default|SetSelectedSlot (Math|Float|Truncate (+ (Variables|Default|GetSelectedSlot) ActionValue)))
      (if (> (Variables|Default|GetSelectedSlot) (- (Variables|/Game/Blueprints/InventorySystem/InventoryComponent.InventoryComponent_C|GetColumns (Variables|Default|GetActionBar1)) 1))
        (Variables|Default|SetSelectedSlot 0)
        (elif (< (Variables|Default|GetSelectedSlot) 0)
          (Variables|Default|SetSelectedSlot (- (Variables|/Game/Blueprints/InventorySystem/InventoryComponent.InventoryComponent_C|GetColumns (Variables|Default|GetActionBar1)) 1)))))
    (:then_1
      (CallFunction|UpdateSelectedSlot))))

(event EventBeginPlay
  (CallFunction|UpdateSelectedSlot))

(event Collision|EventActorBeginOverlap
  (params (OtherActor :type Actor%20Object%20Reference))
  (bind _output_get (Variables|Default|SetOverlappedActor OtherActor))
  (Variables|Default|SetIsInteractableOverlapping (Utilities|DoesObjectImplementInterface _output_get "/Game/Blueprints/BPI_Interactable.BPI_Interactable_C")))

(event EventTick
  (params (DeltaSeconds :type Float%20%28single-precision%29))
  (bind _returnvalue (Game|GetPlayerController 0))
  (bind (_worldlocation _worlddirection) (Game|Player|ConvertMouseLocationToWorldSpace _returnvalue))
  (|CallParentFunction DeltaSeconds)
  (Utilities|FlowControl|Sequence
    (:then_1
      ;[1 1 1] Show / Hide Grid Cells
      (bind (_outhit _returnvalue_2) (Collision|LineTraceForObjects _worldlocation (+ _worldlocation (* _worlddirection 1e+03)) (Utilities|Array|MakeArray "ObjectTypeQuery7") false 0 "None"))
      (if _returnvalue_2
        (Utilities|IsValid (.hitcomponent _outhit) ; Conect from this truee to range in grid
          (:Is%20Valid
            (bind _asstatic_mesh_component (Utilities|Casting|CastToStaticMeshComponent (.hitcomponent _outhit))
              (:then
                (CallFunction|MakePreviousCellInvisible)
                (bind _output_get (Variables|Default|SetSelectedGridCell _asstatic_mesh_component))
                (Rendering|Material|SetScalarParameterValueonMaterials _output_get "Opacity" 0.66))
              (:CastFailed
                (CallFunction|MakePreviousCellInvisible))))
          (:Is%20Not%20Valid
            (CallFunction|MakePreviousCellInvisible)))
        (else
          (CallFunction|MakePreviousCellInvisible))))))

(event Input|MouseEvents|LeftMouseButton
  (params (Key :type Key%20Structure :default "None"))
  (bind _selectedgridcell (Variables|Default|GetSelectedGridCell))
  (bind _returnvalue (Transformation|GetWorldLocation _selectedgridcell))
  (:Pressed
    (bind _asbp_player_controller (Utilities|Casting|CastToBP_PlayerController (Game|GetPlayerController 0)))
    (Utilities|IsValid (Variables|/Script/SC_Project.SCPlayerController|GetGridSetActor _asbp_player_controller)
      (:Is%20Valid
        (Utilities|IsValid _selectedgridcell
          (:Is%20Valid
            (bind (_outhit _returnvalue_2) (Collision|LineTraceForObjects (+ _returnvalue "0.000000,0.000000,64.000000") _returnvalue (Utilities|Array|MakeArray "ObjectTypeQuery2" "ObjectTypeQuery2") false 0 "ForDuration"))
            (if _returnvalue_2
              (bind _asbp_test_block (Utilities|Casting|CastToBP_TestBlock (.HitActor (Collision|BreakHitResult _outhit))))
              (Actor|DestroyActor _asbp_test_block) ; if actor already exist
              (else
                (Game|SpawnActorfromClass "/Game/Blueprints/FarmingSystem/BP_FarmTile.BP_FarmTile_C" (Math|Transform|MakeTransform _returnvalue) "Undefined" "MultiplyWithRoot" 0 0) ; If grid empty, spawn actor
              ))))))))

(event Input|KeyboardEvents|1
  (params (Key :type Key%20Structure :default "None"))
  (:Pressed
    (Default|SetItemInfoatIndex (Variables|Default|GetInventoryComponent) 0 "/Game/Blueprints/InventorySystem/Items/BP_ItemStone.BP_ItemStone_C" 1)
    (Default|SetItemInfoatIndex (Variables|Default|GetInventoryComponent) 1 "/Game/Blueprints/InventorySystem/Items/BP_ItemWood.BP_ItemWood_C" 16)
    (Default|SetItemInfoatIndex (Variables|Default|GetInventoryComponent) 2 "/Game/Blueprints/InventorySystem/Items/BP_ItemWood.BP_ItemWood_C" 8)
    (Default|SetItemInfoatIndex (Variables|Default|GetInventoryComponent) 3 "/Game/Blueprints/InventorySystem/Items/BP_ItemStone.BP_ItemStone_C" 1)
    (Default|SetItemInfoatIndex (Variables|Default|GetInventoryComponent) 4 "/Game/Blueprints/InventorySystem/Items/Consumables/BP_HelathPotion.BP_HelathPotion_C" 3)
    (Default|SetItemInfoatIndex (Variables|Default|GetInventoryComponent) 5 "/Game/Blueprints/InventorySystem/Items/Equipment/BP_SunhatHeadPiece.BP_SunhatHeadPiece_C" 1)
    (Default|SetItemInfoatIndex (Variables|Default|GetInventoryComponent) 6 "/Game/Blueprints/InventorySystem/Items/Equipment/BP_WorkOverallsChestPiece.BP_WorkOverallsChestPiece_C" 1)
    (Default|SetItemInfoatIndex (Variables|Default|GetInventoryComponent) 7 "/Game/Blueprints/InventorySystem/Items/Seeds/BP_WheatSeed.BP_WheatSeed_C" 5)
    (Default|SetItemInfoatIndex (Variables|Default|GetInventoryComponent) 8 "/Game/Blueprints/InventorySystem/Items/Consumables/BP_StaminaPotion.BP_StaminaPotion_C" 5)))

(event Input|KeyboardEvents|I
  (params (Key :type Key%20Structure :default "None"))
  (:Pressed
    (CallFunction|ToggleInventory)))

(event Input|KeyboardEvents|E
  (params (Key :type Key%20Structure :default "None"))
  (:Pressed
    (CallFunction|Interact)
    (Variables|Default|SetInteractKey true))
  (:Released
    (Variables|Default|SetInteractKey false)))

(event Input|KeyboardEvents|AnyKey
  (params (Key :type Key%20Structure :default "None"))
  ;[1 1 1] HotbarNavigation
  (:Pressed
    (CallFunction|HandleKeyboardHotbarInput Key)))

(fn ConstructionScript)

(fn MakePreviousCellInvisible
  (bind _selectedgridcell (Variables|Default|GetSelectedGridCell))
  (Utilities|IsValid _selectedgridcell
    (:Is%20Valid
      (Rendering|Material|SetScalarParameterValueonMaterials _selectedgridcell "Opacity" 0.33))))

(fn ToggleInventory
  (bind _returnvalue (Game|GetPlayerController 0))
  (bind _hudref (Variables|Default|GetHudRef))
  (switch Utilities|FlowControl|Switch|SwitchonESlateVisibility (Widget|GetVisibility (Variables|/Game/Blueprints/UI/Overlay/WBP_InventoryOverlay.WBP_InventoryOverlay_C|GetPlayerInventory (Variables|Default|GetHudRef)))
    (:Visible
      (Widget|SetVisibility (Variables|/Game/Blueprints/UI/Overlay/WBP_InventoryOverlay.WBP_InventoryOverlay_C|GetPlayerInventory (Variables|Default|GetHudRef)) "Hidden")
      (Input|SetInputModeGameOnly _returnvalue false)
      (Variables|/Script/Engine.PlayerController|SetbShowMouseCursor _returnvalue true)
      (Widget|SetVisibility (Variables|/Game/Blueprints/UI/Overlay/WBP_InventoryOverlay.WBP_InventoryOverlay_C|GetCursorIconImage (Variables|Default|GetHudRef)) "Hidden"))
    (:Hidden
      (Widget|SetVisibility (Variables|/Game/Blueprints/UI/Overlay/WBP_InventoryOverlay.WBP_InventoryOverlay_C|GetPlayerInventory (Variables|Default|GetHudRef)) "Visible")
      (Input|SetInputModeGameandUI _returnvalue (Variables|/Game/Blueprints/InventorySystem/Interface/WBP_InventorySlot.WBP_InventorySlot_C|GetSlotButton (CallFunction|GetFirstFocusWidget)) "DoNotLock" false false)
      (Variables|/Script/Engine.PlayerController|SetbShowMouseCursor _returnvalue true)
      (if (Variables|/Game/Blueprints/BP_GameInstance.BP_GameInstance_C|GetDragDrop (Variables|/Game/Blueprints/UI/Overlay/WBP_InventoryOverlay.WBP_InventoryOverlay_C|GetGameInstanceRef _hudref))
        _
        (else
          (Widget|SetVisibility (Variables|/Game/Blueprints/UI/Overlay/WBP_InventoryOverlay.WBP_InventoryOverlay_C|GetCursorIconImage _hudref) "SelfHitTestInvisible")))))
  (Variables|/Script/UMG.WidgetSwitcher|SetActiveWidgetIndex (Variables|/Game/Blueprints/InventorySystem/Interface/WBP_Inventroy.WBP_Inventroy_C|GetWidgetSwitcher_131 (Variables|/Game/Blueprints/UI/Overlay/WBP_InventoryOverlay.WBP_InventoryOverlay_C|GetPlayerInventory (Variables|Default|GetHudRef))) 0))

(fn Interact
  (bind _succes (Class|BPIInteractable|Interacted(Message) (Variables|Default|GetOverlappedActor) self))
  (if _succes
    (return)
    (elif (CallFunction|HoldingConsumableItem)
      (CallFunction|ConsumeItem)
      (elif (CallFunction|HoldingEquipableItem)
        (CallFunction|EquipItem (Variables|Default|GetActionBar1) (Variables|Default|GetSelectedSlot))))))

(fn ToggleStorage
  (bind _returnvalue (Game|GetPlayerController 0))
  (switch Utilities|FlowControl|Switch|SwitchonESlateVisibility (Widget|GetVisibility (Variables|/Game/Blueprints/UI/Overlay/WBP_InventoryOverlay.WBP_InventoryOverlay_C|GetPlayerInventory (Variables|Default|GetHudRef)))
    (:Visible
      (Widget|SetVisibility (Variables|/Game/Blueprints/UI/Overlay/WBP_InventoryOverlay.WBP_InventoryOverlay_C|GetPlayerInventory (Variables|Default|GetHudRef)) "Hidden")
      (Input|SetInputModeGameOnly _returnvalue false)
      (Variables|/Script/Engine.PlayerController|SetbShowMouseCursor _returnvalue true))
    (:Hidden
      (Widget|SetVisibility (Variables|/Game/Blueprints/UI/Overlay/WBP_InventoryOverlay.WBP_InventoryOverlay_C|GetPlayerInventory (Variables|Default|GetHudRef)) "Visible")
      (Input|SetInputModeGameandUI _returnvalue 0 "DoNotLock" false false)
      (Variables|/Script/Engine.PlayerController|SetbShowMouseCursor _returnvalue true)))
  (Variables|/Script/UMG.WidgetSwitcher|SetActiveWidgetIndex (Variables|/Game/Blueprints/InventorySystem/Interface/WBP_Inventroy.WBP_Inventroy_C|GetWidgetSwitcher_131 (Variables|/Game/Blueprints/UI/Overlay/WBP_InventoryOverlay.WBP_InventoryOverlay_C|GetPlayerInventory (Variables|Default|GetHudRef))) 1))

(fn HoldingConsumableItem
  (bind _actionbar1 (Variables|Default|GetActionBar1))
  (bind _selectedslot (Variables|Default|GetSelectedSlot))
  (bind _item (Default|GetItemInfoatIndex _actionbar1 _selectedslot))
  (if (Utilities|IsValidClass _item)
    (switch Utilities|FlowControl|Switch|SwitchonItemCategory (.ItemCategory (Utilities|GetClassDefaults _item))
      (:NewEnumerator0
        _)
      (:NewEnumerator1
        ;[1 1 1] Check for consumable
        (return true))
      (:NewEnumerator2
        _)
      (:NewEnumerator3
        _))
    (return false)
    (else
      (return false))))

(fn ToggleEscapeMenu
  (bind _hudref (Variables|Default|GetHudRef))
  (bind _wbp_escapemenu (Variables|/Game/Blueprints/UI/Overlay/WBP_InventoryOverlay.WBP_InventoryOverlay_C|GetWBP_EscapeMenu _hudref))
  (switch Utilities|FlowControl|Switch|SwitchonESlateVisibility (Widget|GetVisibility (Variables|/Game/Blueprints/UI/Overlay/WBP_InventoryOverlay.WBP_InventoryOverlay_C|GetWBP_EscapeMenu (Variables|Default|GetHudRef)))
    (:Visible
      (Widget|SetVisibility (Variables|/Game/Blueprints/UI/Overlay/WBP_InventoryOverlay.WBP_InventoryOverlay_C|GetWBP_EscapeMenu (Variables|Default|GetHudRef)) "Hidden")
      (Input|SetInputModeGameOnly (Game|GetPlayerController 0) false))
    (:Hidden
      (Widget|SetVisibility _wbp_escapemenu "Visible")
      (Class|WidgetSwitcher|SetActiveWidgetIndex (Variables|/Game/Blueprints/UI/WBP_EscapeMenu.WBP_EscapeMenu_C|GetEscapeMenuWidgetSwitcher _wbp_escapemenu))
      (Input|SetInputModeGameandUI (Game|GetPlayerController 0) (Variables|/Game/Blueprints/UI/WBP_EscapeMenu.WBP_EscapeMenu_C|GetResumeButton _wbp_escapemenu) "DoNotLock" false false))))

(fn GetFirstFocusWidget
  (bind _foundwidgets (Widget|GetAllWidgetsOfClass "/Game/Blueprints/InventorySystem/Interface/WBP_InventorySlot.WBP_InventorySlot_C" false))
  (return (Utilities|Array|Get(acopy) _foundwidgets)))

(fn DropItem
  (params (ItemToDrop :type BP%20Item%20Base%20Class%20Reference) (QuantityToDrop :type Integer))
  (LocalVariables|SetItemToDropLocal ItemToDrop)
  (LocalVariables|SetNewLocalVar QuantityToDrop)
  (Game|SpawnActorfromClass "/Game/Blueprints/InventorySystem/BP_MasterPickUpActor.BP_MasterPickUpActor_C" (Math|Transform|MakeTransform (+ (Transformation|GetActorLocation) (* (Math|Vector|GetForwardVector (Transformation|GetWorldRotation (Variables|Default|GetSprite))) 100)) "0, 0, 0" "1.000000,1.000000,1.000000") "Undefined" "MultiplyWithRoot" 0 (LocalVariables|GetItemToDropLocal) (LocalVariables|GetNewLocalVar) self 0))

(fn UpdateSelectedSlot
  (for _array_element (Variables|/Game/Blueprints/InventorySystem/InventoryComponent.InventoryComponent_C|GetSlotRef (Variables|Default|GetActionBar1))
    (Utilities|IsValid _array_element
      (:Is%20Valid
        (Default|UpdateSelectedSlot _array_element (Variables|Default|GetSelectedSlot)))))
  (CallFunction|HoldItem))

(fn HoldItem
  (bind _actionbar1 (Variables|Default|GetActionBar1))
  (bind _selectedslot (Variables|Default|GetSelectedSlot))
  (bind _itemheld (Variables|Default|GetItemHeld))
  (bind _contents (Variables|/Game/Blueprints/InventorySystem/InventoryComponent.InventoryComponent_C|GetContents _actionbar1))
  (bind _output (Utilities|Array|Get(acopy) _contents _selectedslot))
  (bind (_iteminfo _meshscale) (Utilities|GetClassDefaults (.item _output)))
  (if (Utilities|IsValidClass (.item _output))
    (Components|StaticMesh|SetStaticMesh _itemheld (Utilities|Struct|BreakItemInfo _iteminfo))
    (Transformation|SetWorldScale3D _itemheld _meshscale)
    (else
      (Components|StaticMesh|SetStaticMesh (Variables|Default|GetItemHeld) 0))))

(fn HandleKeyboardHotbarInput
  (params (Key :type Key%20Structure :default "None"))
  (LocalVariables|SetLocalKey Key)
  (bind (_array_element _array_index) (Utilities|Array|ForEachLoopwithBreak (Variables|Default|GetKey) :!label _label)
    (:LoopBody
      (if (== _array_element (LocalVariables|GetLocalKey))
        (goto _label Break)))
    (:Completed
      (if (== _array_element (LocalVariables|GetLocalKey))
        (Variables|Default|SetSelectedSlot _array_index)
        (CallFunction|UpdateSelectedSlot)
        (return)))))

(fn HoldingEquipableItem
  (bind _actionbar1 (Variables|Default|GetActionBar1))
  (bind _selectedslot (Variables|Default|GetSelectedSlot))
  (bind _item (Default|GetItemInfoatIndex _actionbar1 _selectedslot))
  (if (Utilities|IsValidClass _item)
    (switch Utilities|FlowControl|Switch|SwitchonItemCategory (.ItemCategory (Utilities|GetClassDefaults _item))
      (:NewEnumerator0
        _)
      (:NewEnumerator1
        _)
      (:NewEnumerator2
        ;[1 1 1] Check for consumable
        (return true))
      (:NewEnumerator3
        _))
    (return false)
    (else
      (return false))))

(fn EquipItem
  (params (InventoryRef :type Inventory%20Component%20Object%20Reference) (Index :type Integer))
  (bind _playerequipmentcomponent (Variables|Default|GetPlayerEquipmentComponent))
  (bind _contents (Variables|/Game/Blueprints/InventorySystem/InventoryComponent.InventoryComponent_C|GetContents _playerequipmentcomponent))
  (bind _output (Utilities|Array|Get(acopy) _contents))
  (LocalVariables|SetLocalInventoryRef InventoryRef)
  (LocalVariables|SetLocalIndex Index)
  (bind _asbp_equipment_base (Utilities|Casting|CastToBP_EquipmentBaseClass (.Item (Default|GetItemInfoatIndex (LocalVariables|GetLocalInventoryRef) (LocalVariables|GetLocalIndex)))))
  (LocalVariables|SetLocalArmor (.Armor (Utilities|GetClassDefaults _asbp_equipment_base)))
  (LocalVariables|SetLocalHealth (.Helath (Utilities|GetClassDefaults _asbp_equipment_base)))
  (switch Utilities|FlowControl|Switch|SwitchonEquipmentCategory (.EquipmentCategory (Utilities|GetClassDefaults (.Item (Default|GetItemInfoatIndex (LocalVariables|GetLocalInventoryRef) (LocalVariables|GetLocalIndex)))))
    (:NewEnumerator1
      (if (Utilities|IsValidClass (.item (Utilities|Array|Get(acopy) (Variables|/Game/Blueprints/InventorySystem/InventoryComponent.InventoryComponent_C|GetContents (Variables|Default|GetPlayerEquipmentComponent)))))
        (LocalVariables|SetLocalCachedItem (.Item (Default|GetItemInfoatIndex (LocalVariables|GetLocalInventoryRef) (LocalVariables|GetLocalIndex))))
        (LocalVariables|SetLocalCachedQuantity (.Quantity (Default|GetItemInfoatIndex (LocalVariables|GetLocalInventoryRef) (LocalVariables|GetLocalIndex))))
        (Default|SetItemInfoatIndex (LocalVariables|GetLocalInventoryRef) (LocalVariables|GetLocalIndex) (.item _output) (.quantity _output))
        (CallFunction|RemoveStats (.item _output))
        (Default|SetItemInfoatIndex (Variables|Default|GetPlayerEquipmentComponent) (LocalVariables|GetLocalIndex) (LocalVariables|GetLocalCachedItem) (LocalVariables|GetLocalCachedQuantity))
        (else
          (Default|SetItemInfoatIndex (Variables|Default|GetPlayerEquipmentComponent) 0 (.Item (Default|GetItemInfoatIndex (LocalVariables|GetLocalInventoryRef) (LocalVariables|GetLocalIndex))) (.Quantity (Default|GetItemInfoatIndex (LocalVariables|GetLocalInventoryRef) (LocalVariables|GetLocalIndex))))
          (Default|SetItemInfoatIndex (LocalVariables|GetLocalInventoryRef) (LocalVariables|GetLocalIndex))
          ;[1 1 1] Update Player Stats
          (Variables|Default|SetHelath (+ (Variables|Default|GetHelath) (LocalVariables|GetLocalHealth)))
          (Development|PrintString "Hello"))))))

(fn RemoveStats
  (params (Item :type BP%20Item%20Base%20Class%20Reference))
  (bind _hudref (Variables|Default|GetHudRef))
  (bind _playercharacterref (Variables|/Game/Blueprints/UI/Overlay/WBP_InventoryOverlay.WBP_InventoryOverlay_C|GetPlayerCharacterRef _hudref))
  (LocalVariables|SetLocalItem Item)
  (bind _asbp_equipment_base (Utilities|Casting|CastToBP_EquipmentBaseClass (LocalVariables|GetLocalItem)))
  (Variables|BP_SCCharacter_C|SetHelath _playercharacterref (- (Variables|BP_SCCharacter_C|GetHelath _playercharacterref) (.Helath (Utilities|GetClassDefaults _asbp_equipment_base))))
  (return))