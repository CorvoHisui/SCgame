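; BP_MasterLight is a light Blueprint in the day-night cycle folder that fades its point light on or off.
; BeginPlay stores the light's starting intensity, and SwichLight starts a fade only when the requested state differs from the current one.
; Tick steps an alpha over SecondsToSwich to lerp intensity between zero and that stored value.
; Each switch resets alpha to an endpoint, so reversing mid-fade jumps rather than continuing smoothly.
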(event Custom|SwichLightState
  (if (Variables|Default|GetIsLightOn)
    (Variables|Default|SetAlpha 0.0)
    (Variables|Default|SetDirecction 1.0)
    (else
      (Variables|Default|SetAlpha 1.0)
      (Variables|Default|SetDirecction -1.0)))
  (Variables|Default|SetSwichingLight true))

(event EventBeginPlay
  (Variables|Default|SetStartingIntensity (Variables|/Script/Engine.LightComponentBase|GetIntensity (Variables|Default|GetPointLight))))

(event EventSwichLight
  (params (TurnLightOn :type Boolean))
  (if (not (== TurnLightOn (Variables|Default|GetIsLightOn)))
    (Variables|Default|SetIsLightOn TurnLightOn)
    (CallFunction|SwichLightState)))

(event EventTick
  (params (DeltaSeconds :type Float%20%28single-precision%29))
  (if (Variables|Default|GetSwichingLight)
    (Variables|Default|SetAlpha (+ (Variables|Default|GetAlpha) (* (* DeltaSeconds (/ 1.0 (Variables|Default|GetSecondsToSwich))) (Variables|Default|GetDirecction))))
    (Rendering|Components|Light|SetIntensity (Variables|Default|GetPointLight) (Math|Float|Lerp 0.0 (Variables|Default|GetStartingIntensity) (Variables|Default|GetAlpha)))
    (if (> (Variables|Default|GetDirecction) 0.0)
      (if (>= (Variables|Default|GetAlpha) 1.0)
        (Variables|Default|SetSwichingLight false))
      (elif (<= (Variables|Default|GetAlpha) 0.0)
        (Variables|Default|SetSwichingLight false)))))

(fn ConstructionScript)