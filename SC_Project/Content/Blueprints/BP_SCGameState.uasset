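; BP_SCGameState is a game state Blueprint that restores saved farm tiles and provides screen fade helpers.
; SpawnSavedFarmTiles reads SavedPlantStruct from BP_GameInstance, spawns a BP_FarmTile at each saved position and passes it the entry through SpawnFromSave.
; FadeIn and FadeOut each add a new WBP_FadeScene to the viewport and return it with its animation duration.
; Both functions, including FadeOut, call the widget's FadeIn.
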(event Custom|SpawnSavedFarmTiles
  (bind _asbp_game_instance (Utilities|Casting|CastToBP_GameInstance (Game|GetGameInstance)))
  (bind _output_get (Variables|Default|SetAs%20BP%20Game%20Instance _asbp_game_instance))
  (for _array_element (Variables|/Game/Blueprints/BP_GameInstance.BP_GameInstance_C|GetSavedPlantStruct _output_get)
    (bind _returnvalue (Game|SpawnActorfromClass "/Game/Blueprints/FarmingSystem/BP_FarmTile.BP_FarmTile_C" (Math|Transform|MakeTransform (.FarmTilePostion (Utilities|Struct|BreakFPlantInfo _array_element)) "0, 0, 0" "1.000000,1.000000,1.000000") "Undefined" "MultiplyWithRoot" 0 0))
    (Default|SpawnfromSave _returnvalue _array_element)))

(event EventBeginPlay)

(fn ConstructionScript)

(fn Fadein
  (bind _returnvalue (UserInterface|CreateWidget "/Game/Blueprints/UI/WBP_FadeScene.WBP_FadeScene_C"))
  (UserInterface|Viewport|AddtoViewport _returnvalue 0)
  (bind _animationduration (Default|Fadein _returnvalue))
  (return _animationduration _returnvalue))

(fn FadeOut
  (bind _returnvalue (UserInterface|CreateWidget "/Game/Blueprints/UI/WBP_FadeScene.WBP_FadeScene_C"))
  (UserInterface|Viewport|AddtoViewport _returnvalue 0)
  (bind _animationduration (Default|Fadein _returnvalue))
  (return _animationduration _returnvalue))